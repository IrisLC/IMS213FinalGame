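; Cylinder actor that, when overlapped, becomes visible and moves its static mesh vertically in two separately triggered phases.
; The first overlap starts a rise on Tick until the mesh passes an upper world height, where it hides and stops.
; A later overlap shows it again and lowers it until it drops below a lower height, where the actor destroys itself.
; Movement uses fixed per-tick offsets without sweep, so speed depends on frame rate.
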(event `self.ReceiveActorBeginOverlap`
  (params (OtherActor :type "Actor Object Reference"))
  (set `self.canStart` true)
  (`SceneComponent.SetVisibility` (`self.StaticMeshComponent`) true false))

(event `self.ReceiveTick`
  (params (DeltaSeconds :type "Float (single-precision)"))
  (bind _staticmeshcomponent (`self.StaticMeshComponent`))
  (if (`self.canStart`)
    (if (`self.1Done`)
      (`SceneComponent.K2_AddWorldOffset` _staticmeshcomponent (0.0 0.0 -20.0) false false)
      (if (> 200.0 (.z (`SceneComponent.K2_GetComponentLocation` _staticmeshcomponent)))
        (`self.K2_DestroyActor`))
      (else
        (`SceneComponent.K2_AddWorldOffset` _staticmeshcomponent (0.0 0.0 20.0) false false)
        (if (> (.z (`SceneComponent.K2_GetComponentLocation` _staticmeshcomponent)) 1000.0)
          (`SceneComponent.SetVisibility` (`self.StaticMeshComponent`) false false)
          (set `self.canStart` false)
          (set `self.1Done` true))))))

(fn `UserConstructionScript`)