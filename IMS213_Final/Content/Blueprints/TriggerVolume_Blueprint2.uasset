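; Trigger volume that runs a scripted sequence on a wall launcher and two cube actors.
; Overlapping Box starts a scrape sound and slides BP_WallLauncher along Y, then reveals LargeCube_Blueprint and moves it away until destroyed, clearing Done.
; A Box1 overlap while Done is false lowers Cube9_Blueprint, then destroys it and the trigger.
; Tick drives all motion with fixed per-frame offsets, boolean stages and GetActorOfClass lookups.
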(event `self.Box1.OnComponentBeginOverlap`
  (params (OverlappedComponent :type "PrimitiveComponent Object Reference") (OtherActor :type "Actor Object Reference") (OtherComp :type "PrimitiveComponent Object Reference") (OtherBodyIndex :type Integer) (bFromSweep :type Boolean) (SweepResult :type "HitResult Structure (by ref)"))
  (if (not (`self.done`))
    (set `self.beenHit2` true)))

(event `self.Box.OnComponentBeginOverlap`
  (params (OverlappedComponent :type "PrimitiveComponent Object Reference") (OtherActor :type "Actor Object Reference") (OtherComp :type "PrimitiveComponent Object Reference") (OtherBodyIndex :type Integer) (bFromSweep :type Boolean) (SweepResult :type "HitResult Structure (by ref)"))
  (`/Engine/EditorBlueprintResources/StandardMacros.DoOnce` false
    (:`Completed`
      (set `self.beenHit` true)
      (bind _returnvalue (`GameplayStatics.GetActorOfClass` "/Game/Blueprints/BP_WallLauncher.BP_WallLauncher_C"))
      (bind _returnvalue_2 (`GameplayStatics.SpawnSoundAttached` "/Game/Audio/WoodScrape_Cue.WoodScrape_Cue" (`StaticMeshActor.StaticMeshComponent` _returnvalue) "None" (0.0 0.0 0.0) (struct) "KeepRelativeOffset" false 1.0 1.0 0.0 null null)))))

(event `self.ReceiveTick`
  (params (DeltaSeconds :type "Float (single-precision)"))
  (if (`self.beenHit`)
    (if (`self.done`)
      (if (`self.box1done`)
        (bind _returnvalue (`GameplayStatics.GetActorOfClass` "/Game/Blueprints/largeCube_Blueprint.largeCube_Blueprint_C"))
        (`self.K2_AddActorLocalOffset` _returnvalue (0.0 -50.0 0.0) false false)
        (if (< (.y (`self.K2_GetActorLocation` _returnvalue)) -1500.0)
          (set `self.done` false)
          (`self.K2_DestroyActor` _returnvalue))
        (else
          (bind _returnvalue_2 (`GameplayStatics.GetActorOfClass` "/Game/Blueprints/BP_WallLauncher.BP_WallLauncher_C"))
          (`self.K2_AddActorLocalOffset` _returnvalue_2 (0.0 2.0 0.0) false false)
          (if (> (.y (`self.K2_GetActorLocation` _returnvalue_2)) 210.0)
            (set `self.box1done` true)
            (`AudioComponent.Stop` (stale `self.Box.OnComponentBeginOverlap` _returnvalue_2))
            (bind _returnvalue_3 (`GameplayStatics.GetActorOfClass` "/Game/Blueprints/largeCube_Blueprint.largeCube_Blueprint_C"))
            (`SceneComponent.SetVisibility` (`Actor.RootComponent` _returnvalue_3) true false))))
      (elif (`self.beenHit2`)
        (bind _returnvalue_4 (`GameplayStatics.GetActorOfClass` "/Game/Blueprints/Cube9_Blueprint.Cube9_Blueprint_C"))
        (`self.K2_AddActorLocalOffset` _returnvalue_4 (0.0 0.0 -5.0) false false)
        (if (> 100.0 (.z (`self.K2_GetActorLocation` _returnvalue_4)))
          (`self.K2_DestroyActor` _returnvalue_4)
          (`self.K2_DestroyActor`))))))

(fn `UserConstructionScript`)