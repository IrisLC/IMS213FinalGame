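; BP_HiddenFlipper is an actor that flips around its pivot once the player holds a key, then removes itself.
; Any actor overlap checks HasKey on the player's BP_ThirdPersonCharacter and, if set, enables movement after a short delay.
; Tick then rotates PivotPoint by a fixed per-frame step, independent of delta time, and destroys the actor when its pitch exactly equals a target angle.
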(event `self.ReceiveActorBeginOverlap`
  (params (OtherActor :type "Actor Object Reference"))
  (bind _asbp_third_person_character (cast `/Game/ThirdPerson/Blueprints/BP_ThirdPersonCharacter` (`GameplayStatics.GetPlayerCharacter` 0)))
  (if (`/Game/ThirdPerson/Blueprints/BP_ThirdPersonCharacter.hasKey` _asbp_third_person_character)
    (`KismetSystemLibrary.Delay` 0.5)
    (set `self.canMove` true)))

(event `self.ReceiveTick`
  (params (DeltaSeconds :type "Float (single-precision)"))
  (bind _pivotpoint (`self.PivotPoint`))
  (if (`self.canMove`)
    (`SceneComponent.K2_AddLocalRotation` _pivotpoint (struct :`Pitch` 10.0) false false)
    (if (== (.pitch (`SceneComponent.GetSocketRotation` _pivotpoint "None")) -10.0)
      (`self.K2_DestroyActor`))))

(fn `UserConstructionScript`)