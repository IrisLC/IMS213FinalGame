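; BP_WallLauncher is an actor that swings a pivot when something overlaps its trigger Box, apparently as a wall-style launcher.
; The overlap sets DoRotate, and Tick then pitches PivotPoint by a fixed negative step each frame, independent of delta time.
; Rotation stops only when the pivot's world pitch exactly equals -90 degrees, with no logic to return it.
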(event `self.ReceiveTick`
  (params (DeltaSeconds :type "Float (single-precision)"))
  (bind _pivotpoint (`self.PivotPoint`))
  (if (`self.doRotate`)
    (`SceneComponent.K2_AddLocalRotation` _pivotpoint (`KismetMathLibrary.MakeRotator` 0.0 -4.25) false false)
    (if (== (.pitch (`SceneComponent.GetSocketRotation` _pivotpoint "None")) -90.0)
      (set `self.doRotate` false))))

(event `self.Box.OnComponentBeginOverlap`
  (params (OverlappedComponent :type "PrimitiveComponent Object Reference") (OtherActor :type "Actor Object Reference") (OtherComp :type "PrimitiveComponent Object Reference") (OtherBodyIndex :type Integer) (bFromSweep :type Boolean) (SweepResult :type "HitResult Structure (by ref)"))
  (set `self.doRotate` true))

(fn `UserConstructionScript`)