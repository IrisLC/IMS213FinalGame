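; BP_WallPath is an actor, apparently a wall that swings into place as a path, rotating its static mesh when something overlaps it.
; The first overlap, gated by DoOnce, enables movement and plays a low whoosh sound.
; Tick then applies a fixed, frame-rate-dependent local pitch step until the mesh's world pitch reads zero or above, which stops the motion.
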(event `self.ReceiveActorBeginOverlap`
  (params (OtherActor :type "Actor Object Reference"))
  (`/Engine/EditorBlueprintResources/StandardMacros.DoOnce` false
    (:`Completed`
      (set `self.canMove` true)
      (`GameplayStatics.PlaySound2D` "/Game/Audio/LowWoosh.LowWoosh" 1.0 1.0 0.0 null null))))

(event `self.ReceiveTick`
  (params (DeltaSeconds :type "Float (single-precision)"))
  (bind _staticmeshcomponent (`self.StaticMeshComponent`))
  (if (`self.canMove`)
    (`SceneComponent.K2_AddLocalRotation` _staticmeshcomponent (`KismetMathLibrary.MakeRotator` 0.0 -10.0) false false)
    (if (>= (.pitch (`SceneComponent.GetSocketRotation` _staticmeshcomponent "None")) 0.0)
      (set `self.canMove` false))))

(fn `UserConstructionScript`)