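; BP_FlipperPlatform is a platform that flips around a PivotPoint component, triggered by the first actor overlap only.
; The overlap enables Tick-driven rotation, with a Reverse flag selecting a fast swing to an upper roll limit or a slower return to zero.
; Reaching zero stops movement and resets Reverse, while FirstTime stays cleared.
; Rotation uses fixed per-tick steps without delta time, so its speed depends on frame rate.
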(event `self.ReceiveActorBeginOverlap`
  (params (OtherActor :type "Actor Object Reference"))
  (if (`self.firstTime`)
    (set `self.canMove` true)
    (set `self.firstTime` false)))

(event `self.ReceiveTick`
  (params (DeltaSeconds :type "Float (single-precision)"))
  (bind _pivotpoint (`self.PivotPoint`))
  (if (`self.canMove`)
    (if (`self.reverse`)
      (`SceneComponent.K2_AddLocalRotation` _pivotpoint (struct :`Roll` 10.0) false false)
      (if (>= (.roll (`SceneComponent.GetSocketRotation` _pivotpoint "None")) 145.0)
        (set `self.reverse` false))
      (else
        (`SceneComponent.K2_AddLocalRotation` _pivotpoint (struct :`Roll` -0.75) false false)
        (if (<= (.roll (`SceneComponent.GetSocketRotation` _pivotpoint "None")) 0.0)
          (set `self.canMove` false)
          (set `self.reverse` true))))))

(fn `UserConstructionScript`)