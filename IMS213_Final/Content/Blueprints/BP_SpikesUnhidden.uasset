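; Spike trap that springs when an actor overlaps it and kills the player character on contact with its KillZone.
; Overlap plays a movement sound and enables Tick, which slides SpikeHolder along local Z in fixed per-frame steps, using a counter and Reverse flag to bounce and stop.
; KillZone overlaps pass through SpikeCheck, which matches the BP_ThirdPersonCharacter found by class lookup, then destroy it after a short delay.
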(event `self.ReceiveActorBeginOverlap`
  (params (OtherActor :type "Actor Object Reference"))
  (set `self.canMove` true)
  (`GameplayStatics.PlaySoundAtLocation` "/Game/Audio/SpikeMovement_Cue.SpikeMovement_Cue" (0.0 0.0 0.0) (struct) 1.0 1.0 0.0 null null null null))

(event `self.KillZone.OnComponentBeginOverlap`
  (params (OverlappedComponent :type "PrimitiveComponent Object Reference") (OtherActor :type "Actor Object Reference") (OtherComp :type "PrimitiveComponent Object Reference") (OtherBodyIndex :type Integer) (bFromSweep :type Boolean) (SweepResult :type "HitResult Structure (by ref)"))
  (bind _returnvalue (`self.SpikeCheck` OtherActor))
  (if _returnvalue
    (bind _returnvalue_2 (`GameplayStatics.GetActorOfClass` "/Game/ThirdPerson/Blueprints/BP_ThirdPersonCharacter.BP_ThirdPersonCharacter_C"))
    (`KismetSystemLibrary.Delay` 0.2)
    (`self.K2_DestroyActor` _returnvalue_2)))

(event `self.ReceiveTick`
  (params (DeltaSeconds :type "Float (single-precision)"))
  (bind _spikeholder (`self.SpikeHolder`))
  (if (`self.canMove`)
    (if (`self.reverse`)
      (`SceneComponent.K2_AddLocalOffset` _spikeholder (0.0 0.0 5.0) false false)
      (bind _output_get (set `self.counter` (+ (`self.counter`) 5)))
      (if (>= _output_get 120)
        (set `self.reverse` false))
      (else
        (`SceneComponent.K2_AddLocalOffset` _spikeholder (0.0 0.0 -5.0) false false)
        (bind _output_get_2 (set `self.counter` (+ (`self.counter`) -5)))
        (if (<= _output_get_2 0)
          (set `self.reverse` true)
          (set `self.canMove` false))))))

(fn `SpikeCheck`
  (params (self2 :type "Actor Object Reference"))
  (returns (ReturnValue :type Boolean))
  (bind _returnvalue (`GameplayStatics.GetActorOfClass` "/Game/ThirdPerson/Blueprints/BP_ThirdPersonCharacter.BP_ThirdPersonCharacter_C"))
  (return (== (`ActorComponent.GetOwner` (`Actor.RootComponent` self2)) _returnvalue)))

(fn `UserConstructionScript`)