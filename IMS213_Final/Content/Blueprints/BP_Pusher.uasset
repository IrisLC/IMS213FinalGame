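; BP_Pusher is an overlap-triggered moving actor that reveals itself, slides a short distance and disappears.
; Any actor overlap starts a half-second delay, then shows the mesh, enables movement and attaches a wood-scrape sound.
; Tick moves it along local negative X in fixed, unswept steps, so speed depends on frame rate.
; A distance counter stops the sound and destroys the actor after 600 units.
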(event `self.ReceiveActorBeginOverlap`
  (params (OtherActor :type "Actor Object Reference"))
  (`KismetSystemLibrary.Delay` 0.5)
  (`SceneComponent.SetVisibility` (`self.StaticMeshComponent`) true false)
  (set `self.canMove` true)
  (bind _returnvalue (`GameplayStatics.SpawnSoundAttached` "/Game/Audio/WoodScrape_Cue.WoodScrape_Cue" (`self.StaticMeshComponent`) "None" (0.0 0.0 0.0) (struct) "KeepRelativeOffset" false 1.0 1.0 0.0 null null)))

(event `self.ReceiveTick`
  (params (DeltaSeconds :type "Float (single-precision)"))
  (bind _counter (`self.counter`))
  (if (`self.canMove`)
    (`self.K2_AddActorLocalOffset` (-20.0 0.0 0.0))
    (set `self.counter` (+ _counter 20))
    (if (== _counter 600)
      (`AudioComponent.Stop` (stale `self.ReceiveActorBeginOverlap` _returnvalue))
      (`self.K2_DestroyActor`))))

(fn `UserConstructionScript`)