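; Trigger volume Blueprint that makes a Cube12_Blueprint actor sink and disappear once any actor overlaps the volume.
; The overlap sets a BeenTouched flag, which Tick checks alongside Exists.
; Each frame Tick looks up the cube by class and lowers it by a fixed, frame-rate-dependent local offset without sweep.
; When the cube's world Z drops below a threshold, it is destroyed and Exists is cleared.
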(event `self.ReceiveActorBeginOverlap`
  (params (OtherActor :type "Actor Object Reference"))
  (set `self.Been Touched` true))

(event `self.ReceiveTick`
  (params (DeltaSeconds :type "Float (single-precision)"))
  (if (and (`self.exists`) (`self.Been Touched`))
    (bind _returnvalue (`GameplayStatics.GetActorOfClass` "/Game/Blueprints/Cube12_Blueprint.Cube12_Blueprint_C"))
    (`self.K2_AddActorLocalOffset` _returnvalue (0.0 0.0 -5.0) false false)
    (if (< (.z (`self.K2_GetActorLocation` _returnvalue)) 100.0)
      (`self.K2_DestroyActor` _returnvalue)
      (set `self.exists` false))))

(fn `UserConstructionScript`)