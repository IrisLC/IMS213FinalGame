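; Spike trap walkway with two spike groups that rise and retract when triggered and kill the player character.
; Each trigger plays a sound and sets a flag that makes Tick move its cone holder up and down by fixed per-frame steps.
; Both groups share one counter and reverse flag, with the first group taking priority.
; Three kill zones destroy the third-person character after a short delay on overlap.
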(event `self.KillZone1.OnComponentBeginOverlap`
  (params (OverlappedComponent :type "PrimitiveComponent Object Reference") (OtherActor :type "Actor Object Reference") (OtherComp :type "PrimitiveComponent Object Reference") (OtherBodyIndex :type Integer) (bFromSweep :type Boolean) (SweepResult :type "HitResult Structure (by ref)"))
  (`self.SpikeKill` OtherActor))

(event `self.KillZone.OnComponentBeginOverlap`
  (params (OverlappedComponent :type "PrimitiveComponent Object Reference") (OtherActor :type "Actor Object Reference") (OtherComp :type "PrimitiveComponent Object Reference") (OtherBodyIndex :type Integer) (bFromSweep :type Boolean) (SweepResult :type "HitResult Structure (by ref)"))
  (`self.SpikeKill` OtherActor))

(event `self.Trigger1.OnComponentBeginOverlap`
  (params (OverlappedComponent :type "PrimitiveComponent Object Reference") (OtherActor :type "Actor Object Reference") (OtherComp :type "PrimitiveComponent Object Reference") (OtherBodyIndex :type Integer) (bFromSweep :type Boolean) (SweepResult :type "HitResult Structure (by ref)"))
  (set `self.canMove2` true)
  (`GameplayStatics.PlaySoundAtLocation` "/Game/Audio/SpikeMovement_Cue.SpikeMovement_Cue" (0.0 0.0 0.0) (struct) 1.0 1.0 0.0 null null null null))

(event `self.Trigger.OnComponentBeginOverlap`
  (params (OverlappedComponent :type "PrimitiveComponent Object Reference") (OtherActor :type "Actor Object Reference") (OtherComp :type "PrimitiveComponent Object Reference") (OtherBodyIndex :type Integer) (bFromSweep :type Boolean) (SweepResult :type "HitResult Structure (by ref)"))
  (set `self.canMove1` true)
  (`GameplayStatics.PlaySoundAtLocation` "/Game/Audio/SpikeMovement_Cue.SpikeMovement_Cue" (0.0 0.0 0.0) (struct) 1.0 1.0 0.0 null null null null))

(event `self.ReceiveTick`
  (params (DeltaSeconds :type "Float (single-precision)"))
  (bind _coneholder2 (`self.coneHolder2`))
  (bind _coneholder (`self.ConeHolder`))
  (if (`self.canMove1`)
    (if (`self.reverse`)
      (`SceneComponent.K2_AddLocalOffset` _coneholder (0.0 0.0 -5.0) false false)
      (bind _output_get (set `self.counter` (+ (`self.counter`) -5)))
      (if (<= _output_get 0)
        (set `self.canMove1` false)
        (set `self.reverse` false))
      (else
        (`SceneComponent.K2_AddLocalOffset` _coneholder (0.0 0.0 5.0) false false)
        (bind _output_get_2 (set `self.counter` (+ (`self.counter`) 5)))
        (if (>= _output_get_2 90)
          (set `self.reverse` true))))
    (elif (`self.canMove2`)
      (if (`self.reverse`)
        (`SceneComponent.K2_AddLocalOffset` _coneholder2 (0.0 0.0 -5.0) false false)
        (bind _output_get_3 (set `self.counter` (+ (`self.counter`) -5)))
        (if (<= _output_get_3 0)
          (set `self.canMove2` false)
          (set `self.reverse` false))
        (else
          (`SceneComponent.K2_AddLocalOffset` _coneholder2 (0.0 0.0 5.0) false false)
          (bind _output_get_4 (set `self.counter` (+ (`self.counter`) 5)))
          (if (>= _output_get_4 90)
            (set `self.reverse` true)))))))

(event `self.KillZone2.OnComponentBeginOverlap`
  (params (OverlappedComponent :type "PrimitiveComponent Object Reference") (OtherActor :type "Actor Object Reference") (OtherComp :type "PrimitiveComponent Object Reference") (OtherBodyIndex :type Integer) (bFromSweep :type Boolean) (SweepResult :type "HitResult Structure (by ref)"))
  (`self.SpikeKill` OtherActor))

(fn `SpikeCheck`
  (params (self2 :type "Actor Object Reference"))
  (returns (canKill :type Boolean))
  (bind _returnvalue (`GameplayStatics.GetActorOfClass` "/Game/ThirdPerson/Blueprints/BP_ThirdPersonCharacter.BP_ThirdPersonCharacter_C"))
  (return (== (`ActorComponent.GetOwner` (`Actor.RootComponent` self2)) _returnvalue)))

(fn `UserConstructionScript`)