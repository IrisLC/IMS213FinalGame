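; BP_TwisterPlatform1 is a platform that, once triggered, rolls its mesh while driving BP_TwisterPlatform2 in the opposite direction.
; Overlapping the Primer volume arms it, and a later Trigger overlap enables movement and plays a whoosh sound.
; Tick applies fixed per-frame roll steps to both platforms, finding the partner by class each frame, and stops when this mesh's roll exactly equals 90 degrees.
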(event `self.ReceiveTick`
  (params (DeltaSeconds :type "Float (single-precision)"))
  (bind _staticmeshcomponent (`self.StaticMeshComponent`))
  (if (`self.canMove`)
    (`SceneComponent.K2_AddLocalRotation` _staticmeshcomponent (`KismetMathLibrary.MakeRotator` 5.0) false false)
    (bind _returnvalue (`GameplayStatics.GetActorOfClass` "/Game/Blueprints/BP_TwisterPlatform2.BP_TwisterPlatform2_C"))
    (`SceneComponent.K2_AddLocalRotation` (`Actor.RootComponent` _returnvalue) (`KismetMathLibrary.MakeRotator` -5.0) false false)
    (if (== (.roll (`SceneComponent.GetSocketRotation` _staticmeshcomponent "None")) 90.0)
      (set `self.canMove` false))))

(event `self.primer.OnComponentBeginOverlap`
  (params (OverlappedComponent :type "PrimitiveComponent Object Reference") (OtherActor :type "Actor Object Reference") (OtherComp :type "PrimitiveComponent Object Reference") (OtherBodyIndex :type Integer) (bFromSweep :type Boolean) (SweepResult :type "HitResult Structure (by ref)"))
  (set `self.primed` true))

(event `self.trigger.OnComponentBeginOverlap`
  (params (OverlappedComponent :type "PrimitiveComponent Object Reference") (OtherActor :type "Actor Object Reference") (OtherComp :type "PrimitiveComponent Object Reference") (OtherBodyIndex :type Integer) (bFromSweep :type Boolean) (SweepResult :type "HitResult Structure (by ref)"))
  (if (`self.primed`)
    (set `self.canMove` true)
    (`GameplayStatics.PlaySound2D` "/Game/Audio/LowWoosh_Cue.LowWoosh_Cue" 1.0 1.0 0.0 null null)))

(fn `UserConstructionScript`)