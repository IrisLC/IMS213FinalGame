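; Spike trap platform that triggers when an actor overlaps it, playing a spike movement sound at the world origin.
; Tick raises ConeHolder by fixed per-frame steps, tracked by a counter, then lowers it back and stops, so speed depends on frame rate.
; A separate KillZone overlap destroys the other actor after a short delay, skipping the trap itself.
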(event `self.ReceiveActorBeginOverlap`
  (params (OtherActor :type "Actor Object Reference"))
  (set `self.canMove` true)
  (`GameplayStatics.PlaySoundAtLocation` "/Game/Audio/SpikeMovement_Cue.SpikeMovement_Cue" (0.0 0.0 0.0) (struct) 1.0 1.0 0.0 null null null null))

(event `self.ReceiveTick`
  (params (DeltaSeconds :type "Float (single-precision)"))
  (bind _coneholder (`self.ConeHolder`))
  (if (`self.canMove`)
    (if (`self.reverse`)
      (`SceneComponent.K2_AddLocalOffset` _coneholder (0.0 0.0 -10.0) false false)
      (bind _output_get (set `self.counter` (+ (`self.counter`) -10)))
      (if (<= _output_get 0)
        (set `self.canMove` false)
        (set `self.reverse` false))
      (else
        (`SceneComponent.K2_AddLocalOffset` _coneholder (0.0 0.0 10.0) false false)
        (bind _output_get_2 (set `self.counter` (+ (`self.counter`) 10)))
        (if (>= _output_get_2 200)
          (set `self.reverse` true))))))

(event `self.KillZone.OnComponentBeginOverlap`
  (params (OverlappedComponent :type "PrimitiveComponent Object Reference") (OtherActor :type "Actor Object Reference") (OtherComp :type "PrimitiveComponent Object Reference") (OtherBodyIndex :type Integer) (bFromSweep :type Boolean) (SweepResult :type "HitResult Structure (by ref)"))
  (bind _returnvalue (`ActorComponent.GetOwner` (`Actor.RootComponent` OtherActor)))
  (if (not (== _returnvalue (`ActorComponent.GetOwner` (`self.StaticMeshComponent`))))
    (`KismetSystemLibrary.Delay` 0.2)
    (`self.K2_DestroyActor` _returnvalue)))

(fn `UserConstructionScript`)