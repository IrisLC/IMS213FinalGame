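; Sliding pillar actor that, on its first overlap, starts moving apart or together with a second pillar while a wood scrape sound plays.
; Tick shifts it along local -Y and the BP_SlidingPillar2 instance, looked up each frame, along local +Y by fixed, frame-rate-dependent steps.
; When this actor's world Y reaches a hard-coded limit, both stop moving and the sound is cut.
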(event `self.ReceiveActorBeginOverlap`
  (params (OtherActor :type "Actor Object Reference"))
  (`/Engine/EditorBlueprintResources/StandardMacros.DoOnce` false
    (:`Completed`
      (set `self.canMove` true)
      (bind _returnvalue (`GameplayStatics.SpawnSound2D` "/Game/Audio/WoodScrape_Cue.WoodScrape_Cue" 1.0 1.0 0.0 null)))))

(event `self.ReceiveTick`
  (params (DeltaSeconds :type "Float (single-precision)"))
  (if (`self.canMove`)
    (`self.K2_AddActorLocalOffset` (0.0 -10.0 0.0))
    (bind _returnvalue (`GameplayStatics.GetActorOfClass` "/Game/Blueprints/BP_SlidingPillar2.BP_SlidingPillar2_C"))
    (`self.K2_AddActorLocalOffset` _returnvalue (0.0 10.0 0.0) false false)
    (if (<= (.y (`self.K2_GetActorLocation`)) -3100.0)
      (set `self.canMove` false)
      (`AudioComponent.Stop` (stale `self.ReceiveActorBeginOverlap` _returnvalue)))))

(fn `UserConstructionScript`)